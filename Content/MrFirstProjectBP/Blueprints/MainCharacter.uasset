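; MainCharacter is a side-scrolling Paper2D player character, an archer that walks along the X axis and jumps.
; MoveRight input adds movement and snaps controller yaw between 0 and 180 degrees to face the travel direction.
; Each axis update also switches the replicated sprite between walk and idle flipbooks based on velocity.
; BeginPlay enables sprite replication and adds a ResHUD widget to the viewport.
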(event `self.ReceiveBeginPlay`
  ;[1 1 1] Replication
  (`ActorComponent.SetIsReplicated` (`self.Sprite`) true)
  (bind _returnvalue (`|CreateWidget` "/Game/MrFirstProjectBP/Blueprints/ResHUD.ResHUD_C"))
  (bind _output_get (set `self.Game HUDReference` _returnvalue))
  (`UserWidget.AddToViewport` _output_get 0))

(event `InputAxis|MoveRight`
  (params (AxisValue :type "Float (single-precision)"))
  ;[1 1 1] Движение
  (`self.AddMovementInput` (1.0 0.0 0.0) AxisValue)
  (`self.UpdateAnimation`)
  (`/Engine/EditorBlueprintResources/StandardMacros.CompareFloat` AxisValue
    (:`>`
      (`Controller.SetControlRotation` (`self.GetController`) (`KismetMathLibrary.MakeRotator` 0.0)))
    (:`<`
      (`Controller.SetControlRotation` (`self.GetController`) (`KismetMathLibrary.MakeRotator` 0.0 0.0 180.0)))))

(event `InputAction|Jump`
  (params (Key :type "Key Structure" :default "AnyKey"))
  ;[1 1 1] Прыг-Прыг Bitch
  (:`Pressed`
    (`self.Jump`)))

(event `UpdateAnimation`
  (`PaperFlipbookComponent.SetFlipbook` (`self.Sprite`) (select `bool` (> (`KismetMathLibrary.VSize` (`self.GetVelocity`)) 0.0) :`false` "/Game/MrFirstProject/Sprites/Characters/IdleArcher.IdleArcher" :`true` "/Game/MrFirstProject/Sprites/Characters/WalkArcher.WalkArcher" :!type "PaperFlipbook Object Reference")))

(fn `UserConstructionScript`)